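; Base door Blueprint that sets up snapping against other house elements.
; Its construction script collects its right, left, top and bottom points into an array, then passes them to SnappingInit with all actors tagged HouseElement as potential targets.
; GetPoints exposes that point array, and the event graph holds only disabled default events.
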(fn `GetPoints`
  (returns (ArrayPoints :type "Array of SceneComponent Object Reference"))
  (return (`self.ArrayPoints`)))

(fn `UserConstructionScript`
  (`parent.UserConstructionScript`)
  (set `self.ArrayPoints` (`|MakeArray` (`self.RightPoint`) (`self.LeftPoint`) (`self.TopPoint`) (`self.BottomPoint`)))
  (bind _outactors (`GameplayStatics.GetAllActorsWithTag` "HouseElement"))
  (`self.SnappingInit` _outactors (`self.ArrayPoints`)))