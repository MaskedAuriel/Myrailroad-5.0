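; Square intersection Blueprint, likely a base class for house-building pieces, that initializes snapping against other house elements from its Construction Script.
; After running the parent script, it gathers its bottom, top, left and right points into an array.
; It passes that array and all actors tagged HouseElement to SnappingInit.
; GetPoints exposes the point array, and the event graph holds no active logic.
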(fn `GetPoints`
  (returns (ArrayPoints :type "Array of SceneComponent Object Reference"))
  (return (`self.Array Points`)))

(fn `UserConstructionScript`
  (`parent.UserConstructionScript`)
  (set `self.Array Points` (`|MakeArray` (`self.BottomPoint`) (`self.TopPoint`) (`self.LeftPoint`) (`self.RightPoint`)))
  (bind _outactors (`GameplayStatics.GetAllActorsWithTag` "HouseElement"))
  (`self.SnappingInit` _outactors (`self.Array Points`)))