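; Snapping Blueprint for the middle section of a gutter, with a top and a bottom connection point.
; Its construction script runs the parent's script, stores both points in an array, then passes them to SnappingInit with all actors tagged "GutturElement" as potential snap targets.
; GetPoints exposes that point array, and the event graph holds no active logic.
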(fn `GetPoints`
  (returns (ArrayPoints :type "Array of SceneComponent Object Reference"))
  (return (`self.ArrayPoints`)))

(fn `UserConstructionScript`
  (`parent.UserConstructionScript`)
  (set `self.ArrayPoints` (`|MakeArray` (`self.TopPoint`) (`self.BottomPoint`)))
  (bind _outactors (`GameplayStatics.GetAllActorsWithTag` "GutturElement"))
  (`self.SnappingInit` _outactors (`self.ArrayPoints`)))