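; Spline-based train track actor that builds its rails and restarts the level when no turret wagons remain.
; The construction script lays instanced rail meshes along the TrainMovement spline, spaced by the placed mesh's X bounding size.
; Tick searches for BP_Waggon_Turret actors every frame and reopens the current level when none exist.
; MoveTrainPart is an empty stub, and the old wagon-placement logic is deprecated and disconnected.
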(event `self.ReceiveTick`
  (params (DeltaSeconds :type "Float (single-precision)"))
  ;[1 1 1] Check if all turret Wagon are dead
  (bind _outactors (`GameplayStatics.GetAllActorsOfClass` "/Game/Blueprint/Waggon_Related/BP_Waggon_Turret.BP_Waggon_Turret_C"))
  (if (== (`KismetArrayLibrary.Array_Length` _outactors) 0)
    (bind _returnvalue (`GameplayStatics.GetCurrentLevelName` true))
    (`GameplayStatics.OpenLevel` (`KismetStringLibrary.Conv_StringToName` _returnvalue))))

(fn `Get Location at Index`
  (params (A :type Integer))
  (returns (ReturnValue :type "Vector Structure"))
  (return (`SplineComponent.GetLocationAtDistanceAlongSpline` (`self.Train_Movement`) (* A (`self.Spacing bewteween Rail`)) "Local")))

(fn `MoveTrainPart`
  (params (`Train Element` :type "SceneComponent Object Reference") (`Actual Position` :type "Vector Structure")))

(fn `UserConstructionScript`
  (bind _train_movement (`self.Train_Movement`))
  (bind (_min _max) (break `Box` (`StaticMesh.GetBoundingBox` (`self.Placed Mesh`))))
  (bind _returnvalue_x (`KismetMathLibrary.BreakVector` (- _max _min)))
  (`StaticMeshComponent.SetStaticMesh` (`self.Rail`) (`self.Placed Mesh`))
  (bind _output_get (set `self.Spacing bewteween Rail` _returnvalue_x))
  (for _index (range (+ (`KismetMathLibrary.FFloor` (/ (`SplineComponent.GetSplineLength` (`self.Train_Movement`)) _output_get)) 1))
    (bind _returnvalue (* _index (`self.Spacing bewteween Rail`)))
    (`InstancedStaticMeshComponent.AddInstance` (`self.Rail`) (`KismetMathLibrary.MakeTransform` (`SplineComponent.GetLocationAtDistanceAlongSpline` _train_movement _returnvalue "Local") (`SplineComponent.GetRotationAtDistanceAlongSpline` _train_movement _returnvalue "Local")) false)))