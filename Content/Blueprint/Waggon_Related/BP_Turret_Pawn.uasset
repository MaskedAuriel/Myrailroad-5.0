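; Player-controlled turret pawn that rides on a train waggon, aiming and shooting projectiles.
; Axis input turns and pitches the turret core within limits, while Tick zeroes its relative roll to compensate for track tilt.
; Fire alternates between right and left muzzles on a cooldown, launching short-lived projectiles by impulse.
; Switch-side inputs ease the turret between three lateral positions atop the waggon, ignoring input during a move.
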(event `InputAxis|TurnAround`
  (params (AxisValue :type "Float (single-precision)"))
  ;[1 1 1] Camera Movement
  (`SceneComponent.K2_AddWorldRotation` (`self.Turret_Core`) (`KismetMathLibrary.MakeRotator` 0.0 0.0 (`self.GetInputAxisKeyValue`)) false false))

(event `InputAxis|Lookup`
  (params (AxisValue :type "Float (single-precision)"))
  (bind _turret_core (`self.Turret_Core`))
  (bind (_returnvalue_roll _returnvalue_pitch) (`KismetMathLibrary.BreakRotator` (`SceneComponent.K2_GetComponentRotation` _turret_core)))
  ;[1 1 1] Camera Movement
  (bind _asbp_waggon_turret (cast `/Game/Blueprint/Waggon_Related/BP_Waggon_Turret` (`self.GetParentActor` (`ActorComponent.GetOwner` (`self.DefaultSceneRoot`)))))
  (if (> AxisValue 0.0)
    (if (< _returnvalue_pitch 80.0)
      (`SceneComponent.K2_AddLocalRotation` _turret_core (`KismetMathLibrary.MakeRotator` 0.0 (* AxisValue 2.5)) false false :!label _label))
    (elif (> _returnvalue_pitch -20.0)
      (goto _label))))

(event `self.ReceiveTick`
  (params (DeltaSeconds :type "Float (single-precision)"))
  (bind _turret_core (`self.Turret_Core`))
  (bind (_relativerotation_roll _relativerotation_pitch _relativerotation_yaw) (`KismetMathLibrary.BreakRotator` (`SceneComponent.RelativeRotation` _turret_core)))
  ;[1 1 1] Compense Camera Movement on X axis for the turret (Memo : Bad Turret angle when roller coaster)
  (`|ExecutionSequence`
    (:`then_0`
      (`SceneComponent.K2_SetRelativeRotation` _turret_core (`KismetMathLibrary.MakeRotator` 0.0 _relativerotation_pitch _relativerotation_yaw) false false))))

(event `self.ReceiveBeginPlay`
  (bind _returnvalue (`self.GetParentComponent`))
  ;[1 1 1] Pawn Following Train
  (if (== (`GameplayStatics.GetObjectClass` _returnvalue) "/Game/Blueprint/Waggon_Related/BP_Waggon_Turret.BP_Waggon_Turret_C")
    (`SceneComponent.K2_SetWorldLocation` (`self.Turret_Core`) (`SceneComponent.K2_GetComponentLocation` _returnvalue) false false)
    (`self.K2_AttachToComponent` _returnvalue "None" "KeepWorld" "KeepWorld" "KeepWorld")))

(event `InputAction|Fire`
  (params (Key :type "Key Structure"))
  (bind _returnvalue (`GameplayStatics.GetTimeSeconds`))
  ;[1 1 1] Fire
  (:`Pressed`
    (if (>= (- _returnvalue (`self.Time Since Last Shot`)) (`self.Cooldown Between Shot`))
      (set `self.Time Since Last Shot` _returnvalue)
      (`/Engine/EditorBlueprintResources/StandardMacros.FlipFlop`
        (:`A`
          (bind _ball (`self.FireProjectile` (`self.FirePointRight`)))
          (`self.SetLifeSpan` _ball 5.0))
        (:`B`
          (bind _ball_2 (`self.FireProjectile` (`self.FirePointLeft`)))
          (`self.SetLifeSpan` _ball_2 5.0))))))

(event `InputAction|SwitchSideTurretLeft`
  (params (Key :type "Key Structure"))
  ;[1 1 1] Move the turret on the top of a Waggon
  (:`Pressed`
    (if (`self.IsInMovement`)
      _
      (elif (not (== (`self.ActualTurretPosition`) -1))
        (set `self.ActualTurretPosition` (- (`self.ActualTurretPosition`) 1))
        (set `self.IsInMovement` true)
        (`KismetSystemLibrary.MoveComponentTo` (`self.DefaultSceneRoot`) (`KismetMathLibrary.MakeVector` 0.0 (`KismetMathLibrary.Conv_IntToDouble` (* (`self.ActualTurretPosition`) 100))) (struct) false true 1.5)
        (set `self.IsInMovement` false :!label _label_2)))))

(event `InputAction|SwitchSideTurretRight`
  (params (Key :type "Key Structure"))
  ;[1 1 1] Move the turret on the top of a Waggon
  (:`Pressed`
    (if (`self.IsInMovement`)
      _
      (elif (not (== (`self.ActualTurretPosition`) 1))
        (set `self.ActualTurretPosition` (+ (`self.ActualTurretPosition`) 1))
        (set `self.IsInMovement` true)
        (`KismetSystemLibrary.MoveComponentTo` (`self.DefaultSceneRoot`) (`KismetMathLibrary.MakeVector` 0.0 (`KismetMathLibrary.Conv_IntToDouble` (* (`self.ActualTurretPosition`) 100))) (struct) false true 1.5)
        (goto _label_2)))))

(fn `FireProjectile`
  (params (SpawnPoint :type "SceneComponent Object Reference"))
  (returns (Ball :type "Actor Object Reference"))
  (bind (_returnvalue_roll _returnvalue_pitch _returnvalue_yaw) (`KismetMathLibrary.BreakRotator` (`SceneComponent.K2_GetComponentRotation` SpawnPoint)))
  (bind _returnvalue (`|SpawnActorFromClass` "/Game/Blueprint/Waggon_Related/Projectile.Projectile_C" (`KismetMathLibrary.Conv_VectorToTransform` (`SceneComponent.K2_GetComponentLocation` SpawnPoint)) "Undefined" "OverrideRootScale" null null))
  (bind _projectile (`/Game/Blueprint/Waggon_Related/Projectile.Projectile` _returnvalue))
  (`SceneComponent.K2_SetWorldRotation` _projectile (`KismetMathLibrary.MakeRotator` _returnvalue_roll (+ -90.0 _returnvalue_pitch) _returnvalue_yaw) false false)
  (`PrimitiveComponent.AddImpulse` _projectile (* (`KismetMathLibrary.Conv_RotatorToVector` (`KismetMathLibrary.MakeRotator` _returnvalue_roll _returnvalue_pitch _returnvalue_yaw)) (`self.Projectile Impulse`)) "None" true)
  (return _returnvalue))

(fn `UserConstructionScript`)