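; BP_Waggon is a train wagon that rides the spline of its parent BP_Train_Spline actor.
; On BeginPlay a timeline, rate-scaled to the spline's duration and start point, sets location and rotation, offset by wagon order and spacing while HP remains.
; It also caches its child components as snap points.
; DestroyWaggon removes enemies targeting it, then itself; velocity tracking is deprecated and disconnected.
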(event `self.ReceiveBeginPlay`
  (bind _waggon (`self.Waggon`))
  ;[1 1 1] Positionning the Wagon Right on the spline
  (`|ExecutionSequence`
    (:`then_0`
      (bind _asbp_train_spline (cast `/Game/Blueprint/Waggon_Related/BP_Train_Spline` (`self.GetAttachParentActor`)))
      (bind _outactors (`GameplayStatics.GetAllActorsOfClass` "BP_Waggon_C"))
      (bind _returnvalue (/ (`/Game/Blueprint/Waggon_Related/BP_Train_Spline.SplineStartPoint` _asbp_train_spline) 100.0))
      (`TimelineComponent.SetPlayRate` (`self.Train_Moving`) (/ 1.0 (* (`/Game/Blueprint/Waggon_Related/BP_Train_Spline.SplineDurationSeconds` _asbp_train_spline) (- 1.0 _returnvalue))))
      (bind (_direction _movement_train) (`Timeline|Train_Moving` :!via `PlayFromStart`)
        (:`Update`
          (if (not (<= (`self.HPWaggon`) 0.0))
            (bind _train_movement (`/Game/Blueprint/Waggon_Related/BP_Train_Spline.Train_Movement` _asbp_train_spline))
            (bind _returnvalue_2 (`SplineComponent.GetSplineLength` _train_movement))
            (bind _returnvalue_3 (+ (`KismetMathLibrary.Lerp` (* _returnvalue _returnvalue_2) _returnvalue_2 _movement_train) (`KismetMathLibrary.Abs_Int` (* (`/Game/Blueprint/Waggon_Related/BP_Train_Spline.DistanceBetweenWagon` _asbp_train_spline) (- (- (`KismetArrayLibrary.Array_Length` _outactors) 1) (`self.ActualPositionInOrder`))))))
            (`SceneComponent.K2_SetWorldLocation` _waggon (`SplineComponent.GetLocationAtDistanceAlongSpline` _train_movement _returnvalue_3 "World") false false)
            (bind (_returnvalue_roll _returnvalue_pitch _returnvalue_yaw) (`KismetMathLibrary.BreakRotator` (`SplineComponent.GetRotationAtDistanceAlongSpline` _train_movement _returnvalue_3 "World")))
            (`SceneComponent.K2_SetWorldRotation` _waggon (`KismetMathLibrary.MakeRotator` 0.0 _returnvalue_pitch _returnvalue_yaw) false false)))))
    (:`then_1`
      (set `self.ArrayPointSnap` (`SceneComponent.GetChildrenComponents` (`self.Waggon`) false)))))

(event `self.ReceiveTick`
  (params (DeltaSeconds :type "Float (single-precision)"))
  ;[1 1 1] Add Velocity from Train (Deprecated)
)

(event `DestroyWaggon`
  ;[1 1 1] Destroy the Current Waggon
  (bind _outactors (`GameplayStatics.GetAllActorsOfClass` "/Game/Blueprint/Enemy_Related/BP_Enemy.BP_Enemy_C"))
  (for _array_element _outactors
    (if (== (`/Game/Blueprint/Enemy_Related/BP_Enemy.WaggonTargetedComponent` _array_element) self)
      (`self.K2_DestroyActor` _array_element)))
  (`self.K2_DestroyActor` self))

(fn `UserConstructionScript`)