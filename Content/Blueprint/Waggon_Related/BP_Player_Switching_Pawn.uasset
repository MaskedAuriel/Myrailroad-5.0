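; BP_Player_Switching_Pawn handles which pawn the player possesses, cycling between train turrets and toggling an overhead camera.
; On BeginPlay it gathers all BP_Turret_Pawn actors and possesses the first.
; Switching, by input or ForceChangePawn, plays a HUD fade, reattaches BP_CameraAbove to the next turret, and possesses it unless in overhead view.
; A FlipFlop toggles that view; other inputs quit or reload the level.
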(event `self.ReceiveBeginPlay`
  ;[1 1 1] Take first Pawn
  (bind _outactors (`GameplayStatics.GetAllActorsOfClass` "/Game/Blueprint/Waggon_Related/BP_Turret_Pawn.BP_Turret_Pawn_C"))
  (set `self.PawnList` _outactors)
  (set `self.NumberOfPawn` (`KismetArrayLibrary.Array_Length` _outactors))
  (bind _output (`|GetArrayItem` _outactors))
  (`self.Possess` _output)
  (set `self.LastPawn` _output))

(event `ForceChangePawn`
  (bind _output (`|GetArrayItem` (`self.PawnList`) (`self.ActualIndex`)))
  ;[1 1 1] Change Pawn
  (if (not (`KismetSystemLibrary.IsValid` (`|GetArrayItem` (`self.PawnList`) (`self.ActualIndex`)))) :!label _label
    (bind _result (`/Engine/EditorBlueprintResources/StandardMacros.DecrementInt` (`self.NumberOfPawn`))
      (:`  `
        (set `self.NumberOfPawn` _result))))
  (if (> (`self.NumberOfPawn`) 1)
    (bind _asbp_hud_railroad (cast `/Game/Blueprint/Game_Related/BP_HUD_Railroad` (`self.GetHUD` (`GameplayStatics.GetPlayerController` 0))))
    (bind _asfade_in_black (cast `/Game/Blueprint/Widget/FadeInBlack` (`/Game/Blueprint/Game_Related/BP_HUD_Railroad.FadeInBlack` _asbp_hud_railroad)))
    (`/Game/Blueprint/Widget/FadeInBlack.FadeInBlack` _asfade_in_black "Forward")
    (`KismetSystemLibrary.Delay` 0.5)
    (if (not (`self.IsOnTop`))
      (`self.Possess` _output))
    (bind _outactors (`GameplayStatics.GetAllActorsOfClass` "/Game/Blueprint/Waggon_Related/BP_CameraAbove.BP_CameraAbove_C"))
    (`/Game/Blueprint/Waggon_Related/BP_CameraAbove.ReattachTopCamera` (`|GetArrayItem` _outactors) _output)
    (set `self.LastPawn` _output)
    (bind _output_get (set `self.ActualIndex` (+ (`self.ActualIndex`) 1)))
    (if (== _output_get (`self.NumberOfPawn`))
      (set `self.ActualIndex` 0))))

(event `InputAction|ChangeTurret`
  (params (Key :type "Key Structure"))
  ;[1 1 1] Change Pawn
  (:`Pressed`
    (goto _label)))

(event `InputAction|CameraAboveTrain`
  (params (Key :type "Key Structure"))
  ;[1 1 1] Comment
  (:`Pressed`
    (`/Engine/EditorBlueprintResources/StandardMacros.FlipFlop`
      (:`A`
        (bind _outactors (`GameplayStatics.GetAllActorsOfClass` "/Game/Blueprint/Waggon_Related/BP_CameraAbove.BP_CameraAbove_C"))
        (`self.Possess` (`|GetArrayItem` _outactors))
        (set `self.IsOnTop` true))
      (:`B`
        (`self.Possess` (`self.LastPawn`))
        (set `self.IsOnTop` false)))))

(event `InputAction|Close Game`
  (params (Key :type "Key Structure"))
  (:`Pressed`
    (`KismetSystemLibrary.QuitGame` null "Quit")))

(event `InputAction|Reload Map`
  (params (Key :type "Key Structure"))
  (:`Pressed`
    (bind _returnvalue (`GameplayStatics.GetCurrentLevelName` true))
    (`GameplayStatics.OpenLevel` (`KismetStringLibrary.Conv_StringToName` _returnvalue))))

(fn `UserConstructionScript`)