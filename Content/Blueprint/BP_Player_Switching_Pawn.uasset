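; Player switching logic that moves possession between the level's turret pawns and a camera above the train.
; On BeginPlay it caches all BP_Turret_Pawn actors and possesses the first.
; ChangeTurret plays the HUD's fade-to-black, waits briefly, then cycles through the turret list, but is ignored while in the overhead view.
; CameraAboveTrain flip-flops between the BP_CameraAbove pawn and the last turret used.
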(event `self.ReceiveBeginPlay`
  ;[1 1 1] Take first Pawn
  (bind _outactors (`GameplayStatics.GetAllActorsOfClass` "/Game/Blueprint/BP_Turret_Pawn.BP_Turret_Pawn_C"))
  (set `self.PawnList` _outactors)
  (set `self.NumberOfPawn` (`KismetArrayLibrary.Array_Length` _outactors))
  (bind _output (`|GetArrayItem` _outactors))
  (`self.Possess` _output)
  (set `self.LastPawn` _output))

(event `InputAction|ChangeTurret`
  (params (Key :type "Key Structure"))
  (bind _output (`|GetArrayItem` (`self.PawnList`) (`self.ActualIndex`)))
  ;[1 1 1] Change Pawn
  (:`Pressed`
    (if (not (`self.IsOnTop`))
      (bind _asbp_hud_railroad (cast `/Game/Blueprint/BP_HUD_Railroad` (`self.GetHUD` (`GameplayStatics.GetPlayerController` 0))))
      (bind _asfade_in_black (cast `/Game/Blueprint/FadeInBlack` (`/Game/Blueprint/BP_HUD_Railroad.FadeInBlack` _asbp_hud_railroad)))
      (`/Game/Blueprint/FadeInBlack.FadeInBlack` _asfade_in_black "Forward")
      (`KismetSystemLibrary.Delay` 0.5)
      (if (> (`self.NumberOfPawn`) 1)
        (`self.Possess` _output)
        (set `self.LastPawn` _output)
        (bind _output_get (set `self.ActualIndex` (+ (`self.ActualIndex`) 1)))
        (if (== _output_get (`self.NumberOfPawn`))
          (set `self.ActualIndex` 0))))))

(event `InputAction|CameraAboveTrain`
  (params (Key :type "Key Structure"))
  (:`Pressed`
    (`/Engine/EditorBlueprintResources/StandardMacros.FlipFlop`
      (:`A`
        (bind _outactors (`GameplayStatics.GetAllActorsOfClass` "/Game/Blueprint/BP_CameraAbove.BP_CameraAbove_C"))
        (`self.Possess` (`|GetArrayItem` _outactors))
        (set `self.IsOnTop` true))
      (:`B`
        (`self.Possess` (`self.LastPawn`))
        (set `self.IsOnTop` false)))))

(fn `UserConstructionScript`)