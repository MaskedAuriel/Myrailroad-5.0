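; Deprecated parent Blueprint that snaps an actor onto nearby objects by matching snap points.
; SnappingInit compares its own points with those from each other candidate's GetPointsMessage call, stopping further snap attempts after the first success.
; SnappingFunction teleports the whole actor by the offset between two points when they lie within a short fixed distance, and records the result.
; GetPoints is empty here.
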(fn `GetPoints`
  (returns (ArrayPoints :type "Array of SceneComponent Object Reference"))
  (return))

(fn `SnappingFunction`
  (params (PointToSnap :type "SceneComponent Object Reference") (PointApproching :type "SceneComponent Object Reference"))
  (returns (`HasSnap?` :type Boolean))
  (bind _returnvalue (`SceneComponent.K2_GetComponentLocation` PointApproching))
  (bind _returnvalue_2 (`SceneComponent.K2_GetComponentLocation` PointToSnap))
  (if (< (`KismetMathLibrary.Vector_Distance` _returnvalue_2 _returnvalue) 40.0)
    (set `self.HasSnap` true)
    (`self.K2_AddActorWorldOffset` (- _returnvalue _returnvalue_2) false true)
    (else
      (set `self.HasSnap` false)))
  (return (`self.HasSnap`)))

(fn `SnappingInit`
  (params (`List of potential Object` :type "Array of Actor Object Reference") (`Self Points` :type "Array of SceneComponent Object Reference"))
  (for _array_element `List of potential Object`
    (if (!= self _array_element)
      (bind _arraypoints (message `/Game/Blueprint/Deprecated/Snappable.GetPoints` _array_element))
      (for _array_element_2 _arraypoints
        (if (not (`self.HasAlreadSnap`))
          (for _array_element_3 `Self Points`
            (if (not (`self.HasAlreadSnap`))
              (bind _hassnap_ (`self.SnappingFunction` _array_element_3 _array_element_2))
              (set `self.HasAlreadSnap` _hassnap_))))))))

(fn `UserConstructionScript`)