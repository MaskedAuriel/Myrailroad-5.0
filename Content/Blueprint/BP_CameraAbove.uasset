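; BP_CameraAbove is an overhead camera actor that positions itself above a turret pawn.
; On BeginPlay it finds all BP_Turret_Pawn actors and passes the first to the ReattachTopCamera event.
; That event moves the root 3000 units above the given turret.
; It first calls AttachActorToActor with keep-world rules, though no parent actor is shown wired to that call.
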(event `self.ReceiveBeginPlay`
  (bind _outactors (`GameplayStatics.GetAllActorsOfClass` "/Game/Blueprint/BP_Turret_Pawn.BP_Turret_Pawn_C"))
  (`self.ReattachTopCamera` (`|GetArrayItem` _outactors)))

(event `ReattachTopCamera`
  (params (TurretUnder :type "/Game/Blueprint/BP_Turret_Pawn Object Reference"))
  (bind (_returnvalue_x _returnvalue_y _returnvalue_z) (`KismetMathLibrary.BreakVector` (`SceneComponent.K2_GetComponentLocation` (`/Game/Blueprint/BP_Turret_Pawn.DefaultSceneRoot` TurretUnder))))
  (`self.K2_AttachToActor` self null "None" "KeepWorld" "KeepWorld" "KeepWorld" false)
  (`SceneComponent.K2_SetWorldLocation` (`self.DefaultSceneRoot`) (`KismetMathLibrary.MakeVector` _returnvalue_x _returnvalue_y (+ _returnvalue_z 3000.0)) false false))

(fn `UserConstructionScript`)