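; Train wagon actor that travels along the spline of its parent BP_Train_Spline from BeginPlay.
; A timeline, rate-scaled by the spline's duration and start percentage, sets the Wagon's location and rotation from start point to spline end.
; The distance is offset by wagon spacing times an integer parsed from the Wagon's display name.
; It also caches the Wagon's child components in ArrayPointSnap.
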(event `self.ReceiveBeginPlay`
  (bind _wagon (`self.Wagon`))
  (`|ExecutionSequence`
    (:`then_0`
      (bind _asbp_train_spline (cast `/Game/Blueprint/BP_Train_Spline` (`self.GetAttachParentActor`)))
      (bind _returnvalue (/ (`/Game/Blueprint/BP_Train_Spline.SplineStartPoint` _asbp_train_spline) 100.0))
      (`TimelineComponent.SetPlayRate` (`self.Train_Moving`) (/ 1.0 (* (`/Game/Blueprint/BP_Train_Spline.SplineDurationSeconds` _asbp_train_spline) (- 1.0 _returnvalue))))
      (bind (_direction _movement_train) (`Timeline|Train_Moving` :!via `PlayFromStart`)
        (:`Update`
          (bind _train_movement (`/Game/Blueprint/BP_Train_Spline.Train_Movement` _asbp_train_spline))
          (bind _returnvalue_2 (`SplineComponent.GetSplineLength` _train_movement))
          (bind _returnvalue_3 (+ (`KismetMathLibrary.Lerp` (* _returnvalue _returnvalue_2) _returnvalue_2 _movement_train) (`KismetMathLibrary.Abs_Int` (* (`/Game/Blueprint/BP_Train_Spline.DistanceBetweenWagon` _asbp_train_spline) (`KismetStringLibrary.Conv_StringToInt` (`KismetSystemLibrary.GetDisplayName` (`self.Wagon`)))))))
          (`SceneComponent.K2_SetWorldLocation` _wagon (`SplineComponent.GetLocationAtDistanceAlongSpline` _train_movement _returnvalue_3 "World") false false)
          (`SceneComponent.K2_SetWorldRotation` _wagon (`SplineComponent.GetRotationAtDistanceAlongSpline` _train_movement _returnvalue_3 "Local") false false))))
    (:`then_1`
      (set `self.ArrayPointSnap` (`SceneComponent.GetChildrenComponents` (`self.Wagon`) false)))))

(fn `UserConstructionScript`)