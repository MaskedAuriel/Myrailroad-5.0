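; Player-controlled turret pawn that rides on its parent component, noted as the train, and fires physics projectiles.
; On BeginPlay it snaps to and attaches to that parent; axis input then yaws and pitches the turret core, with upward and downward pitch limits.
; Each Fire press alternates right and left muzzles, launching an impulse-driven ball with a limited lifespan.
; A delayed-destroy graph for projectiles exists but is not called here.
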(event `self.ReceiveBeginPlay`
  (bind _returnvalue (`self.GetParentComponent`))
  ;[1 1 1] Pawn Following Train
  (`SceneComponent.K2_SetWorldLocation` (`self.Turret_Core`) (`SceneComponent.K2_GetComponentLocation` _returnvalue) false false)
  (`self.K2_AttachToComponent` _returnvalue "None" "KeepWorld" "KeepWorld" "KeepWorld"))

(event `InputAxis|Lookup`
  (params (AxisValue :type "Float (single-precision)"))
  (bind _turret_core (`self.Turret_Core`))
  (bind (_returnvalue_roll _returnvalue_pitch) (`KismetMathLibrary.BreakRotator` (`SceneComponent.K2_GetComponentRotation` _turret_core)))
  ;[1 1 1] Camera Movement
  (if (> AxisValue 0.0)
    (if (< _returnvalue_pitch 80.0)
      (`SceneComponent.K2_AddLocalRotation` _turret_core (`KismetMathLibrary.MakeRotator` 0.0 (* AxisValue 2.5)) false false :!label _label))
    (elif (> _returnvalue_pitch -20.0)
      (goto _label))))

(event `InputAxis|TurnAround`
  (params (AxisValue :type "Float (single-precision)"))
  ;[1 1 1] Camera Movement
  (`SceneComponent.K2_AddWorldRotation` (`self.Turret_Core`) (`KismetMathLibrary.MakeRotator` 0.0 0.0 (`self.GetInputAxisKeyValue`)) false false))

(event `InputAction|Fire`
  (params (Key :type "Key Structure"))
  ;[1 1 1] Fire
  (:`Pressed`
    (`/Engine/EditorBlueprintResources/StandardMacros.FlipFlop`
      (:`A`
        (bind _ball (`self.FireProjectile` (`self.FirePointRight`)))
        (`self.SetLifeSpan` _ball 5.0))
      (:`B`
        (bind _ball_2 (`self.FireProjectile` (`self.FirePointLeft`)))
        (`self.SetLifeSpan` _ball_2 5.0)))))

(fn `FireProjectile`
  (params (SpawnPoint :type "SceneComponent Object Reference"))
  (returns (Ball :type "Actor Object Reference"))
  (bind _returnvalue (`|SpawnActorFromClass` "/Game/Blueprint/Projectile.Projectile_C" (`KismetMathLibrary.Conv_VectorToTransform` (`SceneComponent.K2_GetComponentLocation` SpawnPoint)) "Undefined" "OverrideRootScale" null null))
  (`PrimitiveComponent.AddImpulse` (`/Game/Blueprint/Projectile.Ball` _returnvalue) (* (`KismetMathLibrary.Conv_RotatorToVector` (`SceneComponent.K2_GetComponentRotation` SpawnPoint)) 7500.0) "None" false)
  (return _returnvalue))

(fn `UserConstructionScript`)