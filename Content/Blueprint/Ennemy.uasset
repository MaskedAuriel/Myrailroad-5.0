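; Enemy actor that attacks a train wagon and is destroyed when projectile hits deplete its HP.
; PlacepointalongtrainSpline moves its spline's endpoint to a predicted point on the train track, using train speed and approach duration.
; LaunchAttack runs Core along that spline, then claims a random non-canon wagon snap point matching the AttackAngle bitmask (left/right/top).
; A second timeline homes Sphere onto the moving point, attaching Core when close.
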(event `Place point along train Spline`
  (bind _ennemymovement (`self.EnnemyMovement`))
  ;[1 1 1] Approxamtively place point alongside Train Spline
  (bind _outactors (`GameplayStatics.GetAllActorsOfClass` "/Game/Blueprint/BP_Train_Spline.BP_Train_Spline_C"))
  (bind _outactors_2 (`GameplayStatics.GetAllActorsOfClass` "/Game/Blueprint/BP_Waggon.BP_Waggon_C"))
  (bind _train_movement (`/Game/Blueprint/BP_Train_Spline.Train_Movement` (`|GetArrayItem` _outactors)))
  (bind _distance (`self.Find Distance Along Spline Closest to World Location` _train_movement (`SceneComponent.K2_GetComponentLocation` (`SceneComponent.GetAttachParent` (`self.DefaultSceneRoot`)))))
  (`SplineComponent.SetLocationAtSplinePoint` _ennemymovement (- (`SplineComponent.GetNumberOfSplinePoints` _ennemymovement) 1) (`SplineComponent.GetLocationAtDistanceAlongSpline` _train_movement (+ (* (/ (`SplineComponent.GetSplineLength` _train_movement) (`TimelineComponent.GetTimelineLength` (`/Game/Blueprint/BP_Waggon.Train_Moving` (`|GetArrayItem` _outactors_2)))) (`TimelineComponent.GetTimelineLength` (`self.MovementOnSpline`))) _distance) "World") "World" true))

(event `LaunchAttack`
  (bind _ennemymovement (`self.EnnemyMovement`))
  (bind _actualpositionwagon (`self.ActualPositionWagon`))
  (bind _returnvalue (`SceneComponent.K2_GetComponentLocation` (`self.Sphere`)))
  (bind _returnvalue_2 (`SceneComponent.K2_GetComponentLocation` (`self.WagonSnapPoint`)))
  (bind _arraypointsnap (`/Game/Blueprint/BP_Waggon.ArrayPointSnap` (`self.WaggonTargetedComponent`)))
  (bind _returnvalue_3 (`KismetMathLibrary.Vector_Distance` _returnvalue _actualpositionwagon))
  (bind _outactors (`GameplayStatics.GetAllActorsOfClass` "/Game/Blueprint/BP_Waggon.BP_Waggon_C"))
  (for _array_element _outactors
    (if (`KismetStringLibrary.EqualEqual_StrStr` (`KismetStringLibrary.Conv_IntToString` (`self.WaggonTargeted`)) (`KismetSystemLibrary.GetDisplayName` _array_element))
      (set `self.WaggonTargetedComponent` _array_element)))
  ;[1 1 1] Launch Movement on Spline
  (`TimelineComponent.SetPlayRate` (`self.MovementOnSpline`) (/ 1.0 (`self.PlayRateInsideSpline`)))
  (bind (_direction _movement_train) (`Timeline|MovementOnSpline` :!via `PlayFromStart`)
    (:`Update`
      (`SceneComponent.K2_SetWorldLocation` (`self.Core`) (`SplineComponent.GetLocationAtDistanceAlongSpline` _ennemymovement (`KismetMathLibrary.Lerp` 0.0 (`SplineComponent.GetSplineLength` _ennemymovement) _movement_train) "World") false false))
    (:`Finished`
      ;[1 1 1] Choosing Snap Point
      (if (!= (`KismetArrayLibrary.Array_Length` (`/Game/Blueprint/BP_Waggon.ArrayPointSnap` (`self.WaggonTargetedComponent`))) 0)
        ;[1 1 1] Check which point to Snap
        (`self.CheckIfTagSnapPoint` "left" (`KismetMathLibrary.Conv_IntToBool` (`KismetMathLibrary.And_IntInt` (`self.AttackAngle`) (`|BitmaskLiteral` 1))))
        (`self.CheckIfTagSnapPoint` "right" (`KismetMathLibrary.Conv_IntToBool` (`KismetMathLibrary.And_IntInt` (`self.AttackAngle`) (`|BitmaskLiteral` 2))))
        (`self.CheckIfTagSnapPoint` "top" (`KismetMathLibrary.Conv_IntToBool` (`KismetMathLibrary.And_IntInt` (`self.AttackAngle`) (`|BitmaskLiteral` 4))))
        (if (!= (`KismetArrayLibrary.Array_Length` (`self.ArrayFinalSnapPoint`)) 0)
          (set `self.RandSnapPoint` (`KismetMathLibrary.RandomInteger` (`KismetArrayLibrary.Array_Length` (`self.ArrayFinalSnapPoint`))))
          (set `self.WagonSnapPoint` (`|GetArrayItem` (`self.ArrayFinalSnapPoint`) (`self.RandSnapPoint`)))
          (for (_array_element_2 _array_index) _arraypointsnap
            (if (== (`self.WagonSnapPoint`) _array_element_2)
              (`KismetArrayLibrary.Array_Remove` _arraypointsnap _array_index)))
          ;[1 1 1] Movement outside Spline
          (set `self.BeginDistance` (`KismetMathLibrary.Vector_Distance` _returnvalue_2 _returnvalue))
          (set `self.ActualPositionWagon` _returnvalue_2)
          (`TimelineComponent.SetPlayRate` (`self.MovementOutsideSpline`) (/ 1.0 (`self.PlayRateOutsideSpline`)))
          (bind (_direction_2 _newtrack_0) (`Timeline|MovementOutsideSpline` :`NewTime` (/ _returnvalue_3 (`self.BeginDistance`)) :!via `PlayFromStart` :!label _label)
            (:`Update`
              (set `self.ActualPositionWagon` (`SceneComponent.K2_GetComponentLocation` (`self.WagonSnapPoint`)))
              (`SceneComponent.K2_SetWorldLocation` (`self.Sphere`) (`KismetMathLibrary.VLerp` _returnvalue _actualpositionwagon _newtrack_0) false false)
              (if (<= _returnvalue_3 5.0)
                (`|ExecutionSequence`
                  (:`then_0`
                    (goto _label :!via `Stop`))
                  (:`then_1`
                    (`SceneComponent.K2_AttachToComponent` (`self.Core`) (`self.WagonSnapPoint`) "None" "KeepWorld" "KeepWorld" "KeepWorld" false)))))))))))

(event `self.Sphere.OnComponentHit`
  (params (HitComponent :type "PrimitiveComponent Object Reference") (OtherActor :type "Actor Object Reference") (OtherComp :type "PrimitiveComponent Object Reference") (NormalImpulse :type "Vector Structure") (Hit :type "HitResult Structure (by ref)"))
  ;[1 1 1] Hit by Projectile
  (bind _asprojectile (cast `/Game/Blueprint/Projectile` OtherActor))
  (bind _output_get (set `self.HP` (- (`self.HP`) (`/Game/Blueprint/Projectile.DamageDone` _asprojectile))))
  (`self.K2_DestroyActor` OtherActor)
  (if (<= _output_get 0)
    (`self.K2_DestroyActor` (`ActorComponent.GetOwner` HitComponent))))

(fn `CheckIfTagSnapPoint`
  (params (`Tag Name` :type String) (BitmaskMatching :type Boolean))
  (if BitmaskMatching
    (for _array_element (`/Game/Blueprint/BP_Waggon.ArrayPointSnap` (`self.WaggonTargetedComponent`))
      (if (`ActorComponent.ComponentHasTag` _array_element (`KismetStringLibrary.Conv_StringToName` `Tag Name`))
        (if (not (`ActorComponent.ComponentHasTag` _array_element "canon"))
          (`KismetArrayLibrary.Array_Add` (`self.ArrayFinalSnapPoint`) _array_element))))))

(fn `Find Distance Along Spline Closest to World Location`
  (params (Spline :type "SplineComponent Object Reference") (WorldLocation :type "Vector Structure"))
  (returns (Distance :type "Float (double-precision)"))
  (bind _returnvalue (`SplineComponent.FindInputKeyClosestToWorldLocation` Spline WorldLocation))
  (bind _returnvalue_2 (`KismetMathLibrary.FTrunc` _returnvalue))
  (bind _returnvalue_3 (`SplineComponent.GetDistanceAlongSplineAtSplinePoint` Spline _returnvalue_2))
  (return (+ _returnvalue_3 (* (- (`SplineComponent.GetDistanceAlongSplineAtSplinePoint` Spline (`KismetMathLibrary.FTrunc` (+ _returnvalue 1.0))) _returnvalue_3) (- _returnvalue (`KismetMathLibrary.Conv_IntToDouble` _returnvalue_2))))))

(fn `UserConstructionScript`
  (bind _ennemymovement (`self.EnnemyMovement`))
  (bind _outactors (`GameplayStatics.GetAllActorsOfClass` "/Game/Blueprint/BP_Train_Spline.BP_Train_Spline_C"))
  (bind _output (`|GetArrayItem` _outactors))
  (bind _train_movement (`/Game/Blueprint/BP_Train_Spline.Train_Movement` _output))
  (bind _distance (`self.Find Distance Along Spline Closest to World Location` _train_movement (`SceneComponent.K2_GetComponentLocation` (`SceneComponent.GetAttachParent` (`self.DefaultSceneRoot`)))))
  (`SplineComponent.SetLocationAtSplinePoint` _ennemymovement (- (`SplineComponent.GetNumberOfSplinePoints` _ennemymovement) 1) (`SplineComponent.GetLocationAtDistanceAlongSpline` (`self.EnnemyMovement`) (+ (* (/ (`SplineComponent.GetSplineLength` _train_movement) (`/Game/Blueprint/BP_Train_Spline.SplineDurationSeconds` _output)) (`TimelineComponent.GetTimelineLength` (`self.MovementOnSpline`))) _distance) "World") "World" true))