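; BP_Train_Spline is an actor with a TrainMovement spline, apparently an unfinished or stripped-down path for a train.
; Its Construction Script prints the distance along the spline at each spline point as debug output.
; BeginPlay and MoveTrainPart are empty stubs, so nothing moves at runtime.
; An unconnected, deprecated wagon-placement chain remains, offsetting the root by wagon spacing along its yaw.
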(event `self.ReceiveBeginPlay`)

(fn `MoveTrainPart`
  (params (`Train Element` :type "SceneComponent Object Reference") (`Actual Position` :type "Vector Structure")))

(fn `UserConstructionScript`
  (bind _train_movement (`self.Train_Movement`))
  (for _index (range (`SplineComponent.GetNumberOfSplinePoints` _train_movement))
    (`KismetSystemLibrary.PrintString` (`KismetStringLibrary.Conv_DoubleToString` (`SplineComponent.GetDistanceAlongSplineAtSplinePoint` _train_movement _index)) true true (struct :`G` 0.66 :`B` 1.0 :`A` 1.0) 7.0)))