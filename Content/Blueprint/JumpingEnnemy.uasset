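; JumpingEnnemy is an enemy Blueprint that moves along a spline path when its LaunchAttack event fires.
; LaunchAttack plays a timeline from the start, mapping its MovementTrain track to a distance along the EnnemyMovement spline.
; Each update places Core at that spline point and sets its world rotation from the spline's local-space rotation, without sweeping the move.
; BeginPlay and construction only call the parent.
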(event `self.ReceiveBeginPlay`
  (`parent.ReceiveBeginPlay`))

(event `LaunchAttack`
  (bind _core (`self.Core`))
  (bind _ennemymovement (`self.EnnemyMovement`))
  (bind (_direction _movement_train) (`Timeline|Timeline_0_0` :!via `PlayFromStart`)
    (:`Update`
      (bind _returnvalue (`KismetMathLibrary.Lerp` 0.0 (`SplineComponent.GetSplineLength` _ennemymovement) _movement_train))
      (`SceneComponent.K2_SetWorldLocation` _core (`SplineComponent.GetLocationAtDistanceAlongSpline` _ennemymovement _returnvalue "World") false false)
      (`SceneComponent.K2_SetWorldRotation` _core (`SplineComponent.GetRotationAtDistanceAlongSpline` _ennemymovement _returnvalue "Local") false false))))

(fn `UserConstructionScript`
  (`parent.UserConstructionScript`))