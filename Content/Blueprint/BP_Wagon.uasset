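; BP_Wagon is a train wagon that moves along the spline of its parent BP_Train_Spline actor.
; On BeginPlay it starts the Train_Moving timeline, whose alpha maps to a distance along the full spline length.
; It offsets that distance by the parent's wagon spacing times an index parsed from the Wagon component's display name.
; Each update sets world location from world-space spline position, but world rotation from local-space spline rotation.
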(event `self.ReceiveBeginPlay`
  (bind _wagon (`self.Wagon`))
  (bind _asbp_train_spline (cast `/Game/Blueprint/BP_Train_Spline` (`self.GetAttachParentActor`)))
  (bind (_direction _movement_train) (`Timeline|Train_Moving` :!via `PlayFromStart`)
    (:`Update`
      (bind _train_movement (`/Game/Blueprint/BP_Train_Spline.Train_Movement` _asbp_train_spline))
      (bind _returnvalue (+ (`KismetMathLibrary.Lerp` 0.0 (`SplineComponent.GetSplineLength` _train_movement) _movement_train) (`KismetMathLibrary.Abs_Int` (* (`/Game/Blueprint/BP_Train_Spline.DistanceBetweenWagon` _asbp_train_spline) (`KismetStringLibrary.Conv_StringToInt` (`KismetSystemLibrary.GetDisplayName` (`self.Wagon`)))))))
      (`SceneComponent.K2_SetWorldLocation` _wagon (`SplineComponent.GetLocationAtDistanceAlongSpline` _train_movement _returnvalue "World") false false)
      (`SceneComponent.K2_SetWorldRotation` _wagon (`SplineComponent.GetRotationAtDistanceAlongSpline` _train_movement _returnvalue "Local") false false))))

(fn `UserConstructionScript`)