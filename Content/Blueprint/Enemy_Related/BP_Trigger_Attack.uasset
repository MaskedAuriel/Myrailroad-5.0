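; BP_Trigger_Attack is a trigger that sends its attached enemies into attack when a designated train wagon reaches it.
; On DetectTrain overlap, it matches the actor's display name against WagonTriggeringTheAttack and sets a flag so it fires once.
; It then calls LaunchAttack on every recursively attached BP_Enemy.
; A helper function, not called here, interpolates between spline points to approximate the distance along a spline closest to a world location.
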(event `self.DetectTrain.OnComponentBeginOverlap`
  (params (OverlappedComponent :type "PrimitiveComponent Object Reference") (OtherActor :type "Actor Object Reference") (OtherComp :type "PrimitiveComponent Object Reference") (OtherBodyIndex :type Integer) (bFromSweep :type Boolean) (SweepResult :type "HitResult Structure (by ref)"))
  (if (`KismetStringLibrary.EqualEqual_StrStr` (`KismetSystemLibrary.GetDisplayName` OtherActor) (`KismetSystemLibrary.GetDisplayName` (`self.WagonTriggeringTheAttack`)))
    (if (not (`self.IsAttackTriggered`))
      (set `self.IsAttackTriggered` true)
      (for _array_element (`self.GetAttachedActors` true true)
        (bind _asbp_enemy (cast `/Game/Blueprint/Enemy_Related/BP_Enemy` _array_element))
        (`/Game/Blueprint/Enemy_Related/BP_Enemy.LaunchAttack` _asbp_enemy)))))

(fn `Find Distance Along Spline Closest to World Location`
  (params (Spline :type "SplineComponent Object Reference") (WorldLocation :type "Vector Structure"))
  (returns (Distance :type "Float (double-precision)"))
  (bind _returnvalue (`SplineComponent.FindInputKeyClosestToWorldLocation` Spline WorldLocation))
  (bind _returnvalue_2 (`KismetMathLibrary.FTrunc` _returnvalue))
  (bind _returnvalue_3 (`SplineComponent.GetDistanceAlongSplineAtSplinePoint` Spline _returnvalue_2))
  (return (+ _returnvalue_3 (* (- (`SplineComponent.GetDistanceAlongSplineAtSplinePoint` Spline (`KismetMathLibrary.FTrunc` (+ _returnvalue 1.0))) _returnvalue_3) (- _returnvalue (`KismetMathLibrary.Conv_IntToDouble` _returnvalue_2))))))

(fn `UserConstructionScript`)