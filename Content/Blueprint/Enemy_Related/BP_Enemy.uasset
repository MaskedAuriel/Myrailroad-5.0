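; Enemy that attacks a train wagon and takes damage from projectiles.
; Its spline end is placed at the predicted point on the train track from train speed and travel time.
; On LaunchAttack, timelines move it along that spline, then home onto a random free snap point filtered by the AttackAngle bitmask.
; Once attached, Tick drains wagon HP on a cooldown, then destroys wagon and enemy and forces a player pawn switch.
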(event `Place point along train Spline`
  (bind _ennemymovement (`self.EnnemyMovement`))
  ;[1 1 1] Approxamtively place point alongside Train Spline
  (bind _outactors (`GameplayStatics.GetAllActorsOfClass` "/Game/Blueprint/Waggon_Related/BP_Train_Spline.BP_Train_Spline_C"))
  (bind _output (`|GetArrayItem` _outactors))
  (bind _train_movement (`/Game/Blueprint/Waggon_Related/BP_Train_Spline.Train_Movement` _output))
  (bind _distance (`self.Find Distance Along Spline Closest to World Location` _train_movement (`SceneComponent.K2_GetComponentLocation` (`SceneComponent.GetAttachParent` (`self.DefaultSceneRoot`)))))
  (`SplineComponent.SetLocationAtSplinePoint` _ennemymovement (- (`SplineComponent.GetNumberOfSplinePoints` _ennemymovement) 1) (`SplineComponent.GetLocationAtDistanceAlongSpline` _train_movement (+ (* (/ (`SplineComponent.GetSplineLength` _train_movement) (`/Game/Blueprint/Waggon_Related/BP_Train_Spline.SplineDurationSeconds` _output)) (`self.PlayRateInsideSpline`)) _distance) "World") "World" true))

(event `LaunchAttack`
  (bind _ennemymovement (`self.EnnemyMovement`))
  (bind _actualpositionwagon (`self.ActualPositionWagon`))
  (bind _waggontargetedcomponent (`self.WaggonTargetedComponent`))
  (bind _returnvalue (`SceneComponent.K2_GetComponentLocation` (`self.Core`)))
  (bind _returnvalue_2 (`SceneComponent.K2_GetComponentLocation` (`self.WagonSnapPoint`)))
  (bind _arraypointsnap (`/Game/Blueprint/Waggon_Related/BP_Waggon.ArrayPointSnap` (`self.WaggonTargetedComponent`)))
  (bind _returnvalue_3 (`KismetMathLibrary.Vector_Distance` _returnvalue _actualpositionwagon))
  ;[1 1 1] LaunchAttack
  (set `self.WaggonTargetedComponent` (`self.WagonTargetedBP`))
  ;[1 1 1] Launch Movement on Spline
  (`TimelineComponent.SetPlayRate` (`self.MovementOnSpline`) (/ 1.0 (`self.PlayRateInsideSpline`)))
  (bind (_direction _movement_train) (`Timeline|MovementOnSpline` :!via `PlayFromStart`)
    (:`Update`
      (`SceneComponent.K2_SetWorldLocation` (`self.Core`) (`SplineComponent.GetLocationAtDistanceAlongSpline` _ennemymovement (`KismetMathLibrary.Lerp` 0.0 (`SplineComponent.GetSplineLength` _ennemymovement) _movement_train) "World") false false))
    (:`Finished`
      ;[1 1 1] Choosing Snap Point
      (if (`KismetSystemLibrary.IsValid` _waggontargetedcomponent)
        (if (`self.WagonDestroyed`)
          _
          (elif (!= (`KismetArrayLibrary.Array_Length` (`/Game/Blueprint/Waggon_Related/BP_Waggon.ArrayPointSnap` _waggontargetedcomponent)) 0)
            ;[1 1 1] Check which point to Snap
            (`self.CheckIfTagSnapPoint` "left" (`KismetMathLibrary.Conv_IntToBool` (`KismetMathLibrary.And_IntInt` (`self.AttackAngle`) (`|BitmaskLiteral` 1))))
            (`self.CheckIfTagSnapPoint` "right" (`KismetMathLibrary.Conv_IntToBool` (`KismetMathLibrary.And_IntInt` (`self.AttackAngle`) (`|BitmaskLiteral` 2))))
            (`self.CheckIfTagSnapPoint` "top" (`KismetMathLibrary.Conv_IntToBool` (`KismetMathLibrary.And_IntInt` (`self.AttackAngle`) (`|BitmaskLiteral` 4))))
            (if (!= (`KismetArrayLibrary.Array_Length` (`self.ArrayFinalSnapPoint`)) 0)
              (set `self.RandSnapPoint` (`KismetMathLibrary.RandomInteger` (`KismetArrayLibrary.Array_Length` (`self.ArrayFinalSnapPoint`))))
              (set `self.WagonSnapPoint` (`|GetArrayItem` (`self.ArrayFinalSnapPoint`) (`self.RandSnapPoint`)))
              (for (_array_element _array_index) _arraypointsnap
                (if (== (`self.WagonSnapPoint`) _array_element)
                  (`KismetArrayLibrary.Array_Remove` _arraypointsnap _array_index)))
              ;[1 1 1] Movement outside Spline
              (set `self.BeginDistance` (`KismetMathLibrary.Vector_Distance` _returnvalue_2 (`SceneComponent.K2_GetComponentLocation` (`self.Sphere`))))
              (set `self.ActualPositionWagon` _returnvalue_2)
              (`TimelineComponent.SetPlayRate` (`self.MovementOutsideSpline`) (/ 1.0 (`self.PlayRateOutsideSpline`)))
              (bind (_direction_2 _newtrack_0) (`Timeline|MovementOutsideSpline` :`NewTime` (/ _returnvalue_3 (`self.BeginDistance`)) :!via `PlayFromStart` :!label _label)
                (:`Update`
                  (set `self.ActualPositionWagon` (`SceneComponent.K2_GetComponentLocation` (`self.WagonSnapPoint`)))
                  (`SceneComponent.K2_SetWorldLocation` (`self.Core`) (`KismetMathLibrary.VLerp` _returnvalue _actualpositionwagon _newtrack_0) false false)
                  (if (<= _returnvalue_3 20.0)
                    (`|ExecutionSequence`
                      (:`then_0`
                        (goto _label :!via `Stop`))
                      (:`then_1`
                        (`SceneComponent.K2_AttachToComponent` (`self.Core`) (`self.WagonSnapPoint`) "None" "KeepWorld" "KeepWorld" "KeepWorld" false)
                        (set `self.CanMakeDamage` true)))))))))))))

(event `self.ReceiveTick`
  (params (DeltaSeconds :type "Float (single-precision)"))
  (bind _waggontargetedcomponent (`self.WaggonTargetedComponent`))
  ;[1 1 1] Do Damage On train
  (if (`self.WagonDestroyed`)
    _
    (elif (`self.CanMakeDamage`)
      (if (>= (`/Game/Blueprint/Waggon_Related/BP_Waggon.HPWaggon` _waggontargetedcomponent) 0.0)
        (`self.DoDamageOnTrain` _waggontargetedcomponent)
        (else
          (`self.K2_DestroyActor` self)
          (`/Game/Blueprint/Waggon_Related/BP_Waggon.DestroyWaggon` (`self.WaggonTargetedComponent`))
          (bind _asbp_player_switching_pawn (cast `/Game/Blueprint/Waggon_Related/BP_Player_Switching_Pawn` (`GameplayStatics.GetPlayerController` 0)))
          (`/Game/Blueprint/Waggon_Related/BP_Player_Switching_Pawn.ForceChangePawn` _asbp_player_switching_pawn)
          (set `self.WagonDestroyed` true)
          (set `self.CanMakeDamage` false))))))

(event `self.Sphere.OnComponentHit`
  (params (HitComponent :type "PrimitiveComponent Object Reference") (OtherActor :type "Actor Object Reference") (OtherComp :type "PrimitiveComponent Object Reference") (NormalImpulse :type "Vector Structure") (Hit :type "HitResult Structure (by ref)"))
  ;[1 1 1] Hit by Projectile
  (bind _asprojectile (cast `/Game/Blueprint/Waggon_Related/Projectile` OtherActor))
  (bind _output_get (set `self.HPEnemy` (- (`self.HPEnemy`) (`/Game/Blueprint/Waggon_Related/Projectile.DamageDone` _asprojectile))))
  (`self.K2_DestroyActor` OtherActor)
  (if (<= _output_get 0.0)
    (`self.K2_DestroyActor` (`ActorComponent.GetOwner` HitComponent))))

(event `self.Sphere.OnComponentBeginOverlap`
  (params (OverlappedComponent :type "PrimitiveComponent Object Reference") (OtherActor :type "Actor Object Reference") (OtherComp :type "PrimitiveComponent Object Reference") (OtherBodyIndex :type Integer) (bFromSweep :type Boolean) (SweepResult :type "HitResult Structure (by ref)"))
  ;[1 1 1] Hit by Projectile
  (bind _asprojectile (cast `/Game/Blueprint/Waggon_Related/Projectile` OtherActor))
  (bind _output_get (set `self.HPEnemy` (- (`self.HPEnemy`) (`/Game/Blueprint/Waggon_Related/Projectile.DamageDone` _asprojectile))))
  (`self.K2_DestroyActor` OtherActor)
  (if (<= _output_get 0.0)
    (`self.K2_DestroyActor` (`ActorComponent.GetOwner` OverlappedComponent))))

(fn `CheckIfTagSnapPoint`
  (params (`Tag Name` :type String) (BitmaskMatching :type Boolean))
  (if BitmaskMatching
    (for _array_element (`/Game/Blueprint/Waggon_Related/BP_Waggon.ArrayPointSnap` (`self.WaggonTargetedComponent`))
      (if (`ActorComponent.ComponentHasTag` _array_element (`KismetStringLibrary.Conv_StringToName` `Tag Name`))
        (if (not (`ActorComponent.ComponentHasTag` _array_element "inactive"))
          (`KismetArrayLibrary.Array_Add` (`self.ArrayFinalSnapPoint`) _array_element))))))

(fn `DoDamageOnTrain`
  (params (WagonToAttack :type "/Game/Blueprint/Waggon_Related/BP_Waggon Object Reference"))
  (bind _returnvalue (`GameplayStatics.GetTimeSeconds`))
  (if (>= (- _returnvalue (`self.TimeSinceLastAttack`)) (`self.Cooldown`))
    (set `self.TimeSinceLastAttack` _returnvalue)
    (set `/Game/Blueprint/Waggon_Related/BP_Waggon.HPWaggon` (- (`/Game/Blueprint/Waggon_Related/BP_Waggon.HPWaggon` WagonToAttack) (`self.DamageDoneOnWaggon`)) WagonToAttack)))

(fn `Find Distance Along Spline Closest to World Location`
  (params (Spline :type "SplineComponent Object Reference") (WorldLocation :type "Vector Structure"))
  (returns (Distance :type "Float (double-precision)"))
  (bind _returnvalue (`SplineComponent.FindInputKeyClosestToWorldLocation` Spline WorldLocation))
  (bind _returnvalue_2 (`KismetMathLibrary.FTrunc` _returnvalue))
  (bind _returnvalue_3 (`SplineComponent.GetDistanceAlongSplineAtSplinePoint` Spline _returnvalue_2))
  (return (+ _returnvalue_3 (* (- (`SplineComponent.GetDistanceAlongSplineAtSplinePoint` Spline (`KismetMathLibrary.FTrunc` (+ _returnvalue 1.0))) _returnvalue_3) (- _returnvalue (`KismetMathLibrary.Conv_IntToDouble` _returnvalue_2))))))

(fn `UserConstructionScript`
  (bind _ennemymovement (`self.EnnemyMovement`))
  (bind _outactors (`GameplayStatics.GetAllActorsOfClass` "/Game/Blueprint/Waggon_Related/BP_Train_Spline.BP_Train_Spline_C"))
  (bind _output (`|GetArrayItem` _outactors))
  (bind _train_movement (`/Game/Blueprint/Waggon_Related/BP_Train_Spline.Train_Movement` _output))
  (bind _distance (`self.Find Distance Along Spline Closest to World Location` _train_movement (`SceneComponent.K2_GetComponentLocation` (`SceneComponent.GetAttachParent` (`self.DefaultSceneRoot`)))))
  (`SplineComponent.SetLocationAtSplinePoint` _ennemymovement (- (`SplineComponent.GetNumberOfSplinePoints` _ennemymovement) 1) (`SplineComponent.GetLocationAtDistanceAlongSpline` (`self.EnnemyMovement`) (+ (* (/ (`SplineComponent.GetSplineLength` _train_movement) (`/Game/Blueprint/Waggon_Related/BP_Train_Spline.SplineDurationSeconds` _output)) (`TimelineComponent.GetTimelineLength` (`self.MovementOnSpline`))) _distance) "World") "World" true))